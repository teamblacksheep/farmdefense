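; Blueprint function library of global helpers for game manager access, UI visibility and cursor control.
; Get Game Manager casts the current game mode to DGameMode and returns its GameManager.
; Hide UI sets every top-level user widget to hidden.
; Show Mouse toggles the first player controller's cursor and switches input mode between UI-only, without mouse lock, and game-only to match.
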(fn `Get Game Manager`
  (returns (`Game Manager` :type "/Game/__MyContent/Blueprints/Asset_BP/GameManager Object Reference"))
  (bind _asdgame_mode (cast `/Game/__MyContent/Blueprints/Asset_BP/DGameMode` (`GameplayStatics.GetGameMode` null)))
  (return (`/Game/__MyContent/Blueprints/Asset_BP/DGameMode.Game Manager` _asdgame_mode)))

(fn `Hide UI`
  (bind _foundwidgets (`WidgetBlueprintLibrary.GetAllWidgetsOfClass` null "/Script/UMG.UserWidget"))
  (for _array_element _foundwidgets
    (`Widget.SetVisibility` _array_element "Hidden")))

(fn `Show Mouse`
  (params (visible :type Boolean))
  (bind _returnvalue (`GameplayStatics.GetPlayerController` null))
  (bind _output_get (set `PlayerController.bShowMouseCursor` visible _returnvalue))
  (if _output_get
    (`WidgetBlueprintLibrary.SetInputMode_UIOnlyEx` _returnvalue null)
    (else
      (`WidgetBlueprintLibrary.SetInputMode_GameOnly` _returnvalue))))