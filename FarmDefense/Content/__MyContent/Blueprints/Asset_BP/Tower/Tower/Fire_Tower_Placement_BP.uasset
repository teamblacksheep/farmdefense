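; Placement preview actor for the fire tower, which follows the mouse cursor until the player places it.
; Each tick, it traces under the cursor against WorldStatic objects and moves itself to the hit location.
; On the Place Tower input, if the cursor is over an actor of exact class BP_Wall, it spawns Fire_Turret_BP at its own transform and destroys itself.
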(event `self.ReceiveTick`
  (params (DeltaSeconds :type "Float (single-precision)"))
  (bind (_hitresult _returnvalue) (`PlayerController.GetHitResultUnderCursorForObjects` (`GameplayStatics.GetPlayerController` 0) (`|MakeArray` "ObjectTypeQuery1" :!type "EObjectTypeQuery Enum") true))
  (if _returnvalue
    (`self.K2_SetActorLocation` (`.Location` (`GameplayStatics.BreakHitResult` _hitresult)))))

(event `InputAction|Place Tower`
  (params (Key :type "Key Structure"))
  (:`Pressed`
    (if (== (`GameplayStatics.GetObjectClass` (`.HitActor` (`GameplayStatics.BreakHitResult` (`PlayerController.GetHitResultUnderCursorForObjects` (`GameplayStatics.GetPlayerController` 0) (`|MakeArray` "ObjectTypeQuery1" :!type "EObjectTypeQuery Enum") true)))) "/Game/__MyContent/Blueprints/BP_Wall.BP_Wall_C")
      (`|SpawnActorFromClass` "/Game/__MyContent/Blueprints/Asset_BP/Tower/Tower/Fire_Turret_BP.Fire_Turret_BP_C" (`self.GetTransform`) "Undefined" "OverrideRootScale" null null null)
      (`self.K2_DestroyActor`))))

(fn `UserConstructionScript`)