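; Base turret Blueprint that targets any TopDownCharacter entering its TargetingRadius.
; Begin overlap stores the character as Target, enables locking and spawns a single Tower_Projectile_BP at the turret's transform, passing it the target.
; While locked, Tick rotates Tower1Gun toward the target in pitch and yaw with zero roll.
; Any actor leaving the radius clears the lock, with no check that it is the current target.
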(event `self.Targeting Radius.OnComponentBeginOverlap`
  (params (OverlappedComponent :type "PrimitiveComponent Object Reference") (OtherActor :type "Actor Object Reference") (OtherComp :type "PrimitiveComponent Object Reference") (OtherBodyIndex :type Integer) (bFromSweep :type Boolean) (SweepResult :type "HitResult Structure (by ref)"))
  (bind _astop_down_character (cast `/Game/__MyContent/Blueprints/TopDownCharacter` OtherActor))
  (set `self.Targetlocking` true)
  (bind _output_get (set `self.Target` _astop_down_character))
  (`|SpawnActorFromClass` "/Game/__MyContent/Blueprints/Asset_BP/Tower/Tower/Tower_Projectile_BP.Tower_Projectile_BP_C" (`self.GetTransform`) "Undefined" "OverrideRootScale" null _output_get null))

(event `self.Targeting Radius.OnComponentEndOverlap`
  (params (OverlappedComponent :type "PrimitiveComponent Object Reference") (OtherActor :type "Actor Object Reference") (OtherComp :type "PrimitiveComponent Object Reference") (OtherBodyIndex :type Integer))
  (set `self.Targetlocking` false))

(event `self.ReceiveTick`
  (params (DeltaSeconds :type "Float (single-precision)"))
  ;[1 1 1] Rotation and target locking
  (if (`self.Targetlocking`)
    (`self.update turret rotation`)))

(event `update turret rotation`
  ;[1 1 1] Rotation and target locking
  (`SceneComponent.K2_SetWorldRotation` (`self.Tower1_Gun`) (`KismetMathLibrary.MakeRotator` 0.0 (.pitch (`KismetMathLibrary.FindLookAtRotation` (`SceneComponent.K2_GetComponentLocation` (`self.Tower1_Gun`)) (`self.K2_GetActorLocation` (`self.Target`)))) (.yaw (`KismetMathLibrary.FindLookAtRotation` (`SceneComponent.K2_GetComponentLocation` (`self.Tower1_Gun`)) (`self.K2_GetActorLocation` (`self.Target`))))) false false))

(fn `UserConstructionScript`)