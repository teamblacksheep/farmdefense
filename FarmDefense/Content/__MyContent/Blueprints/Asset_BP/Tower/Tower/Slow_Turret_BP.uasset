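; Slow turret for a tower defense game that shoots at TestDummy targets within its radius.
; BeginPlay loads the Ice_Tower data table row; TowerInit applies its meshes and range.
; Sphere overlaps maintain a target list, and Tick aims the gun at the first entry while firing when ready.
; The row's projectile type selects a standard or slowing projectile, with cooldown set by fire rate times the GameManager's slow-tower speed.
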(event `self.Targeting Radius.OnComponentBeginOverlap`
  (params (OverlappedComponent :type "PrimitiveComponent Object Reference") (OtherActor :type "Actor Object Reference") (OtherComp :type "PrimitiveComponent Object Reference") (OtherBodyIndex :type Integer) (bFromSweep :type Boolean) (SweepResult :type "HitResult Structure (by ref)"))
  ;[1 1 1] Firing Code
  (`/Engine/EditorBlueprintResources/StandardMacros.IsValid` (`self.Enemy`)
    (:`Is Not Valid`
      (bind _astest_dummy (cast `/Game/__MyContent/Blueprints/AI/TestDummy` OtherActor))
      (`KismetArrayLibrary.Array_Add` (`self.Target`) _astest_dummy)
      (set `self.Targetlocking` true))))

(event `CanFire`
  (bind _returnvalue (`self.GetTransform`))
  (bind (_name _damage _range _firerate _basemesh _gunmesh _projectile) (break `/Game/__MyContent/Blueprints/Asset_BP/Tower/Tower/Tower_Struct` (`self.TowerStruct`)))
  (bind _output (`|GetArrayItem` (`self.Target`)))
  ;[1 1 1] Firing Code
  (set `self.CanFire?` true)
  (switch `/Game/__MyContent/Blueprints/Asset_BP/Tower/Tower/ProjectileTypes` _projectile
    (:`NewEnumerator0`
      (`|SpawnActorFromClass` "/Game/__MyContent/Blueprints/Asset_BP/Tower/Tower/Tower_Projectile_BP.Tower_Projectile_BP_C" _returnvalue "Undefined" "OverrideRootScale" null _output null))
    (:`NewEnumerator1`
      (`|SpawnActorFromClass` "/Game/__MyContent/Blueprints/Asset_BP/Tower/Tower/Tower_Projectile_BPslow.Tower_Projectile_BPslow_C" _returnvalue "Undefined" "OverrideRootScale" null _output null)))
  (set `self.CanFire?` false)
  (bind _game_manager (`/Game/__MyContent/Blueprints/Asset_BP/FucntionLibrary.Get Game Manager`))
  (`KismetSystemLibrary.Delay` (* _firerate (`/Game/__MyContent/Blueprints/Asset_BP/GameManager.SlowTower_Speed` _game_manager)))
  (set `self.CanFire?` true))

(event `self.Targeting Radius.OnComponentEndOverlap`
  (params (OverlappedComponent :type "PrimitiveComponent Object Reference") (OtherActor :type "Actor Object Reference") (OtherComp :type "PrimitiveComponent Object Reference") (OtherBodyIndex :type Integer))
  (bind _target (`self.Target`))
  ;[1 1 1] Firing Code
  (for _array_element _target
    (set `self.Targetlocking` false)
    (if (== OtherActor _array_element)
      (`KismetArrayLibrary.Array_RemoveItem` _target _array_element))))

(event `self.ReceiveBeginPlay`
  (bind _returnvalue (`|GetDataTableRow` "/Game/__MyContent/Blueprints/Asset_BP/Tower/Tower/Tower_Data_Table.Tower_Data_Table" "Ice_Tower")
    (:`then`
      (set `self.TowerStruct` _returnvalue))))

(event `self.ReceiveTick`
  (params (DeltaSeconds :type "Float (single-precision)"))
  ;[1 1 1] Firing Code
  (`/Engine/EditorBlueprintResources/StandardMacros.IsValid` (`|GetArrayItem` (`self.Target`))
    (:`Is Valid`
      (`self.update turret rotation`)
      (if (`self.CanFire?`)
        (`self.CanFire`)))))

(event `update turret rotation`
  ;[1 1 1] Rotation and target locking
  (`SceneComponent.K2_SetWorldRotation` (`self.Tower1_Gun`) (`KismetMathLibrary.MakeRotator` 0.0 (.pitch (`KismetMathLibrary.FindLookAtRotation` (`SceneComponent.K2_GetComponentLocation` (`self.Tower1_Gun`)) (`self.K2_GetActorLocation` (`|GetArrayItem` (`self.Target`))))) (.yaw (`KismetMathLibrary.FindLookAtRotation` (`SceneComponent.K2_GetComponentLocation` (`self.Tower1_Gun`)) (`self.K2_GetActorLocation` (`|GetArrayItem` (`self.Target`)))))) false false))

(event `TowerInit`
  (bind (_name _damage _range _firerate _basemesh _gunmesh) (break `/Game/__MyContent/Blueprints/Asset_BP/Tower/Tower/Tower_Struct` (`self.TowerStruct`)))
  ;[1 1 1] Tower Struct Logic
  (`StaticMeshComponent.SetStaticMesh` (`self.Tower1_Base`) _basemesh)
  (`StaticMeshComponent.SetStaticMesh` (`self.Tower1_Gun`) _gunmesh)
  (`SphereComponent.SetSphereRadius` (`self.Targeting Radius`) _range true))

(fn `UserConstructionScript`)