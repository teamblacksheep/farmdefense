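; Game manager Blueprint that holds the current game state and switches the UI to match it.
; On BeginPlay it enters Init, which creates the HUD, game over, pause, menu, enemy health and how-to-play widgets, then moves to Start.
; SetState hides all UI, then shows the state's widget or HUD and sets mouse visibility.
; Only Start pauses the game and Running unpauses it; Pause and Lost leave pausing untouched.
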(event `self.ReceiveBeginPlay`
  (`self.Set State` "NewEnumerator4"))

(fn `Create UI`
  (bind _returnvalue (`|CreateWidget` "/Game/__MyContent/Blueprints/UI/Main_Overlay_Widget.Main_Overlay_Widget_C"))
  (bind _output_get (set `self.Main_Overlay_Widget` _returnvalue))
  (`UserWidget.AddToViewport` _output_get 0)
  (bind _returnvalue_2 (`|CreateWidget` "/Game/__MyContent/Blueprints/UI/Widget_GameOver.Widget_GameOver_C"))
  (bind _output_get_2 (set `self.Widget GAme Over` _returnvalue_2))
  (`UserWidget.AddToViewport` _output_get_2 -1)
  (bind _returnvalue_3 (`|CreateWidget` "/Game/__MyContent/Blueprints/UI/Widget_Pause.Widget_Pause_C"))
  (bind _output_get_3 (set `self.Widget Pause` _returnvalue_3))
  (`UserWidget.AddToViewport` _output_get_3 0)
  (bind _returnvalue_4 (`|CreateWidget` "/Game/__MyContent/Blueprints/UI/Widget_Menu.Widget_Menu_C"))
  (bind _output_get_4 (set `self.Widget Menu` _returnvalue_4))
  (`UserWidget.AddToViewport` _output_get_4 0)
  (bind _returnvalue_5 (`|CreateWidget` "/Game/__MyContent/Blueprints/UI/EnemyHealth.EnemyHealth_C"))
  (bind _output_get_5 (set `self.EnemyHealth` _returnvalue_5))
  (`UserWidget.AddToViewport` _output_get_5 0)
  (bind _returnvalue_6 (`|CreateWidget` "/Game/__MyContent/Blueprints/UI/Widget_HowToPlay.Widget_HowToPlay_C"))
  (bind _output_get_6 (set `self.How2Play` _returnvalue_6))
  (`UserWidget.AddToViewport` _output_get_6 0))

(fn `Get State`
  (returns (state :type "/Game/__MyContent/Blueprints/Asset_BP/My_Game_state Enum"))
  (return (`self.Current game State`)))

(fn `Init`
  (`self.Create UI`)
  (`self.Set State` "NewEnumerator8"))

(fn `Set State`
  (params (`New State` :type "/Game/__MyContent/Blueprints/Asset_BP/My_Game_state Enum" :default "NewEnumerator0"))
  (`/Game/__MyContent/Blueprints/Asset_BP/FucntionLibrary.Hide UI`)
  (bind _output_get (set `self.Current game State` `New State`))
  (switch `/Game/__MyContent/Blueprints/Asset_BP/My_Game_state` _output_get
    (:`NewEnumerator0`
      (`/Game/__MyContent/Blueprints/Asset_BP/FucntionLibrary.Show Mouse` false)
      (`self.Show HUD` true)
      (`GameplayStatics.SetGamePaused` false))
    (:`NewEnumerator2`
      (`Widget.SetVisibility` (`self.Widget GAme Over`) "Visible")
      (`/Game/__MyContent/Blueprints/Asset_BP/FucntionLibrary.Show Mouse` true :!label _label))
    (:`NewEnumerator3`
      (`Widget.SetVisibility` (`self.Widget Pause`) "Visible")
      (goto _label))
    (:`NewEnumerator4`
      (`self.Init`))
    (:`NewEnumerator8`
      (`/Game/__MyContent/Blueprints/Asset_BP/FucntionLibrary.Show Mouse` true)
      (`Widget.SetVisibility` (`self.Widget Menu`) "Visible")
      (`GameplayStatics.SetGamePaused` true))))

(fn `Show HUD`
  (params (visible :type Boolean))
  (bind _main_overlay_widget (`self.Main_Overlay_Widget`))
  (if visible
    (`Widget.SetVisibility` _main_overlay_widget "Visible")
    (else
      (`Widget.SetVisibility` _main_overlay_widget "Hidden"))))

(fn `UserConstructionScript`)