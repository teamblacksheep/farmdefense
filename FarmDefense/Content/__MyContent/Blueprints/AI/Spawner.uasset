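; Enemy wave spawner that runs the wave countdown and changes the Game Manager state once wave 40 is reached and no enemies remain.
; Tick with a one-second Delay counts down the manager's timer, starting the next wave at zero.
; Each wave reads its Runner_Data_Table row and spawns TestDummy AI in a delayed loop, applying health, speed, mesh and currency drop while incrementing the manager's enemy count.
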(event `self.ReceiveTick`
  (params (DeltaSeconds :type "Float (single-precision)"))
  (`KismetSystemLibrary.Delay` 1.0)
  ;[1 1 1] Win condition (wave # + enemy actor hit 0)
  (if (== (`self.wave`) 40)
    (bind _game_manager (`/Game/__MyContent/Blueprints/Asset_BP/FucntionLibrary.Get Game Manager`))
    (set `/Game/__MyContent/Blueprints/Asset_BP/GameManager.WaveTimer` 0 _game_manager)
    (if (== (`/Game/__MyContent/Blueprints/Asset_BP/GameManager.CurrentEnemy` _game_manager) 0)
      (`/Game/__MyContent/Blueprints/Asset_BP/GameManager.Set State` _game_manager "NewEnumerator1"))
    (else
      ;[1 1 1] Wave Timer
      (bind _game_manager_2 (`/Game/__MyContent/Blueprints/Asset_BP/FucntionLibrary.Get Game Manager`))
      (`/Engine/EditorBlueprintResources/StandardMacros.DecrementInt` (`/Game/__MyContent/Blueprints/Asset_BP/GameManager.WaveTimer` _game_manager_2)
        (:`  `
          (if (== (`/Game/__MyContent/Blueprints/Asset_BP/GameManager.WaveTimer` _game_manager_2) 0)
            (set `self.initialTimer` false)
            (`self.Next wave`)
            (bind _game_manager_3 (`/Game/__MyContent/Blueprints/Asset_BP/FucntionLibrary.Get Game Manager`))
            (set `/Game/__MyContent/Blueprints/Asset_BP/GameManager.WaveTimer` 60 _game_manager_3)))))))

(event `Next wave`
  (`self.INCWaveCount`)
  (set `self.SpawnCount` 1)
  (bind _returnvalue (`|GetDataTableRow` "/Game/__MyContent/Blueprints/Wave/Runner_Data_Table.Runner_Data_Table" (`KismetStringLibrary.Conv_StringToName` (`KismetStringLibrary.Conv_IntToString` (`self.wave`))))
    (:`then`
      (bind (_name _health _runspeed _enemycount _currencydrop _mash) (break `/Game/__MyContent/Blueprints/Wave/Runner_structure` _returnvalue))
      ;[1 1 1] Spawn enemy till = spawn table
      (if (not (> (`self.SpawnCount`) _enemycount)) :!label _label
        (bind _returnvalue_2 (`AIBlueprintHelperLibrary.SpawnAIFromClass` "/Game/__MyContent/Blueprints/AI/TestDummy.TestDummy_C" null (`self.K2_GetActorLocation`)))
        (bind _astest_dummy (cast `/Game/__MyContent/Blueprints/AI/TestDummy` _returnvalue_2))
        ;[1 1 1] Current Enemy Counter on spawn
        (bind _game_manager (`/Game/__MyContent/Blueprints/Asset_BP/FucntionLibrary.Get Game Manager`))
        (set `/Game/__MyContent/Blueprints/Asset_BP/GameManager.CurrentEnemy` (+ (`/Game/__MyContent/Blueprints/Asset_BP/GameManager.CurrentEnemy` _game_manager) 1) _game_manager)
        (set `/Game/__MyContent/Blueprints/AI/TestDummy.Spawner` self _astest_dummy)
        ;[1 1 1] CurrencyDrop
        (set `/Game/__MyContent/Blueprints/AI/TestDummy.CurrencyDrop` _currencydrop _astest_dummy)
        ;[1 1 1] Enemy Actor HP
        (bind _output_get (set `/Game/__MyContent/Blueprints/AI/TestDummy.Max HP` _health _astest_dummy))
        (set `/Game/__MyContent/Blueprints/AI/TestDummy.Health Points` _output_get _astest_dummy)
        ;[1 1 1] Enemy Actor walk speed
        (bind _output_get_2 (set `CharacterMovementComponent.MaxWalkSpeed` _runspeed (`Character.CharacterMovement` _astest_dummy)))
        (set `/Game/__MyContent/Blueprints/AI/TestDummy.default walk speed` _output_get_2 _astest_dummy)
        ;[1 1 1] Set enemy Skin
        (`SkinnedMeshComponent.SetSkinnedAssetAndUpdate` (`Character.Mesh` _astest_dummy) _mash true)
        ;[1 1 1] Spawn count
        (`/Engine/EditorBlueprintResources/StandardMacros.IncrementInt` (`self.SpawnCount`)
          (:`  `
            ;[1 1 1] Delay between enemy spawn
            (`KismetSystemLibrary.Delay` 1.0)
            (goto _label)))))))

(fn `INCWaveCount`
  (bind _output_get (set `self.wave` (+ (`self.wave`) 1)))
  (bind _game_manager (`/Game/__MyContent/Blueprints/Asset_BP/FucntionLibrary.Get Game Manager`))
  (set `/Game/__MyContent/Blueprints/Asset_BP/GameManager.CurrentWAve` (- _output_get 0) _game_manager))

(fn `UserConstructionScript`)