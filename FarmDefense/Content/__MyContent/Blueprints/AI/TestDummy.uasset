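; TestDummy is an AI test target that holds a health value and reports it to an enemy health display.
; Set Health caps the points at 100 and, while they stay above zero, writes the normalised value to EnemyHealth on the Game Manager.
; Change Health applies deltas through Set Health, and Init starts the dummy at half health.
; The event graph is empty, and reaching zero triggers no death logic.
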(fn `Change Health`
  (params (`Delta Points` :type "Float (double-precision)"))
  (`self.Set Health` (+ `Delta Points` (`self.Health Points`))))

(fn `Get Health`
  (returns (`Health Points` :type "Float (double-precision)"))
  (return (`self.Health Points`)))

(fn `Init`
  (`self.Set Health` 50.0))

(fn `Set Health`
  (params (`Health Points` :type "Float (double-precision)"))
  (bind _output_get (set `self.Health Points` `Health Points`))
  (if (> _output_get 100.0)
    (set `self.Health Points` 100.0))
  (if (not (<= _output_get 0.0))
    (bind _game_manager (`/Game/__MyContent/Blueprints/Asset_BP/FucntionLibrary.Get Game Manager`))
    (set `/Game/__MyContent/Blueprints/UI/EnemyHealth.Health` (/ (`self.Health Points`) 100.0) (`/Game/__MyContent/Blueprints/Asset_BP/GameManager.EnemyHealth` _game_manager))))

(fn `UserConstructionScript`)