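; TDPlayer is a player actor that provides mouse edge-scroll panning, likely for a top-down camera.
; Each Tick compares player 0's mouse position with the outer ten percent of the viewport to set PanLeft and PanUp directions.
; When either is nonzero, it offsets its location along world X and Y by PanningSpeed per frame, without delta-time scaling or sweep.
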(event `self.ReceiveTick`
  (params (DeltaSeconds :type "Float (single-precision)"))
  (bind _panningspeed (`self.PanningSpeed`))
  (bind (_x _y) (`KismetMathLibrary.BreakVector2D` (`WidgetLayoutLibrary.GetViewportSize`)))
  (bind _x_2 (`KismetMathLibrary.BreakVector2D` (`WidgetLayoutLibrary.GetViewportSize`)))
  (bind (_locationx _locationy) (`PlayerController.GetMousePosition` (`GameplayStatics.GetPlayerController` 0)))
  (if (< _locationx (* _x_2 0.1))
    (set `self.PanLeft` -1)
    (elif (> _locationx (* _x_2 0.9))
      (set `self.PanLeft` 1)
      (else
        (set `self.PanLeft` 0))))
  (if (< _locationy (* _y 0.1))
    (set `self.PanUp` 1)
    (elif (> _locationy (* _y 0.9))
      (set `self.PanUp` -1)
      (else
        (set `self.PanUp` 0))))
  (if (or (!= (`self.PanLeft`) 0) (!= (`self.PanUp`) 0))
    (`self.K2_SetActorLocation` (+ (`self.K2_GetActorLocation`) (`KismetMathLibrary.MakeVector` (* (`self.PanUp`) _panningspeed) (* (`self.PanLeft`) _panningspeed))))))

(fn `UserConstructionScript`)